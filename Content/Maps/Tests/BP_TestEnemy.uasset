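; BP_TestEnemy is a test enemy actor whose cube mesh shows a time-driven glow effect.
; On BeginPlay it creates a dynamic material instance from M_TestEnemy on the cube.
; Each Tick accumulates time alive and feeds it into the GlowCycle scalar parameter, printing an error if the material cast fails.
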(event `self.ReceiveBeginPlay`
  (`PrimitiveComponent.CreateDynamicMaterialInstance` (`self.Cube`) 0 "/Game/Maps/Tests/M_TestEnemy.M_TestEnemy"))

(event `self.ReceiveTick`
  (params (DeltaSeconds :type "Float (single-precision)"))
  (bind _output_get (set `self.TimeAlive` (+ (`self.TimeAlive`) DeltaSeconds)))
  (bind _asmaterial_instance_dynamic (cast `MaterialInstanceDynamic` (`PrimitiveComponent.GetMaterial` (`self.Cube`) 0))
    (:`then`
      (`MaterialInstanceDynamic.SetScalarParameterValue` _asmaterial_instance_dynamic "GlowCycle" _output_get))
    (:`CastFailed`
      (`KismetSystemLibrary.PrintString` "Material cast failed!" true true (struct :`R` 1.0 :`B` 0.029831 :`A` 1.0)))))

(fn `UserConstructionScript`
  (`parent.UserConstructionScript`))