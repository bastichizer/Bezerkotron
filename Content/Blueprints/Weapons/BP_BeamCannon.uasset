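; BP_BeamCannon is a weapon scene component that fires a continuous, damaging beam.
; BeginPlay creates inactive beam and impact-spark emitters, which FireBeam and StopFiring reuse, toggling component tick alongside.
; While firing, each tick line-traces forward against world static and dynamic objects, moves sparks to the hit and spawns a short-lived burn decal.
; Hit actors implementing BPI_DamageTaker take base damage every tick, so damage depends on frame rate.
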(event `self.ReceiveBeginPlay`
  (set `self.parent` (`self.GetOwner`))
  (bind _returnvalue (`GameplayStatics.SpawnEmitterAttached` "/Game/Particles/P_BlastGun.P_BlastGun" self (`self.GetAttachSocketName`) (0.0 0.0 0.0) (struct) "SnapToTarget" false))
  (bind _output_get (set `self.BeamEmitter` _returnvalue))
  (`self.Deactivate` _output_get)
  (bind _returnvalue_2 (`GameplayStatics.SpawnEmitterAtLocation` "/Game/Particles/P_BeamImpactSparks.P_BeamImpactSparks" (0.0 0.0 0.0) (struct) false))
  (bind _output_get_2 (set `self.BeamImpactSparks` _returnvalue_2))
  (`self.Deactivate` _output_get_2))

(event `self.ReceiveTick`
  (params (DeltaSeconds :type "Float (single-precision)"))
  (bind _beamimpactsparks (`self.BeamImpactSparks`))
  (bind _returnvalue (`self.K2_GetComponentLocation` self))
  (if (`self.isFiring`)
    (bind (_outhit _returnvalue_2) (`KismetSystemLibrary.LineTraceSingleForObjects` _returnvalue (+ _returnvalue (* (`self.GetForwardVector`) 50000.0)) (`|MakeArray` "ObjectTypeQuery1" "ObjectTypeQuery2" :!type "EObjectTypeQuery Enum")))
    (bind _output_get (set `self.BeamHit` _returnvalue_2))
    (if _output_get
      (bind (_bblockinghit _binitialoverlap _time _location _impactpoint _normal _impactnormal _physmat _hitactor) (`GameplayStatics.BreakHitResult` _outhit))
      (`self.K2_SetWorldLocation` _beamimpactsparks _impactpoint false false)
      (`self.K2_SetWorldRotation` _beamimpactsparks (`KismetMathLibrary.MakeRotFromZ` _impactnormal) false false)
      (`self.Activate` _beamimpactsparks false)
      (`GameplayStatics.SpawnDecalAtLocation` "/Game/Materials/M_BlastImpactBurn.M_BlastImpactBurn" (100.0 100.0 100.0) _impactpoint (`KismetMathLibrary.MakeRotFromZ` (* _impactnormal -1.0)) 5.0)
      (bind _asbpi_damage_taker (cast `/Game/Blueprints/Interfaces/Combat/BPI_DamageTaker` _hitactor))
      (`/Game/Blueprints/Interfaces/Combat/BPI_DamageTaker.ApplyDamage` _asbpi_damage_taker (`KismetMathLibrary.Conv_ByteToInt` (`self.weaponType`)) (`self.baseDamage`))
      (else
        (`self.Deactivate` _beamimpactsparks)))))

(event `self.FireBeam`
  (`self.Activate` (`self.BeamEmitter`) false)
  (set `self.isFiring` true)
  (`self.SetComponentTickEnabled` true))

(fn `StopFiring`
  (`self.Deactivate` (`self.BeamEmitter`))
  (set `self.isFiring` false)
  (`self.SetComponentTickEnabled` false)
  (set `self.BeamHit` false)
  (`self.Deactivate` (`self.BeamImpactSparks`)))