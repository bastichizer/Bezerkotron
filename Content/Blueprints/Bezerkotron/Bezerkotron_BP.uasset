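; Bezerkotron is the player-possessed flying vehicle pawn, which constantly moves forward and fires two beam cannons while the primary fire input is held.
; Tick applies roll, pitch and yaw either directly from input or through a HUD steering widget that accumulates clamped mouse movement as a virtual stick.
; A crosshair widget follows a distant forward point from the Transmorpher's vehicle-mode neck socket, projected to screen space.
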(event `self.ReceiveBeginPlay`
  (bind _returnvalue (`GameplayStatics.GetPlayerController` 0))
  ;[1 1 1] Set player control of Bezerkotron
  (`PlayerController.SetViewTargetWithBlend` _returnvalue self 0.0 "VTBlend_Linear" 0.0 false)
  (`Controller.Possess` _returnvalue self)
  (bind _returnvalue_2 (`|CreateWidget` "/Game/Blueprints/UI/HUD/HUD_SteeringIndicator.HUD_SteeringIndicator_C" _returnvalue))
  (bind _output_get (set `self.HUD_SteeringWidget` _returnvalue_2))
  (`UserWidget.AddToViewport` _output_get 0)
  (bind _returnvalue_3 (`|CreateWidget` "/Game/Blueprints/UI/HUD/HUD_Crosshair.HUD_Crosshair_C" _returnvalue))
  (bind _output_get_2 (set `self.HUD_Crosshair` _returnvalue_3))
  (bind _screenpos (`self.GetScreenSpaceAimPoint`))
  (`/Game/Blueprints/UI/HUD/HUD_Crosshair.SetCrosshairPosition` _output_get_2 _screenpos)
  (`UserWidget.AddToViewport` _output_get_2 0))

(event `self.ReceiveTick`
  (params (DeltaSeconds :type "Float (single-precision)"))
  (if (`self.HUD_Steering`)
    ;[1 1 1] Set attitude (HUD control)
    (bind _steervector (`/Game/Blueprints/UI/HUD/HUD_SteeringIndicator.GetSteerVector` (`self.HUD_SteeringWidget`)))
    (bind (_x _y) (`KismetMathLibrary.BreakVector2D` _steervector))
    (`self.K2_AddActorLocalRotation` (* (`KismetMathLibrary.MakeRotator` (* (`self.GetInputAxisValue`) (`self.RollSpeed`)) (* _y -1.0) _x) DeltaSeconds))
    (else
      ;[1 1 1] Set attitude (direct control)
      (`self.K2_AddActorLocalRotation` (* (`KismetMathLibrary.MakeRotator` (* (`self.GetInputAxisValue`) (`self.RollSpeed`)) (* (`self.GetInputAxisValue`) (`self.PitchSpeed`)) (* (`self.GetInputAxisValue`) (`self.YawSpeed`))) DeltaSeconds))))
  ;[1 1 1] Translate
  (`self.K2_AddActorWorldTransform` (`KismetMathLibrary.Conv_VectorToTransform` (* (* (`self.GetActorForwardVector`) (`self.MaxSpeed`)) DeltaSeconds)))
  (`self.AddMouseInputToHUD`)
  (bind _screenpos (`self.GetScreenSpaceAimPoint`))
  (`/Game/Blueprints/UI/HUD/HUD_Crosshair.SetCrosshairPosition` (`self.HUD_Crosshair`) _screenpos))

(event `InputAction|Fire_1`
  (params (Key :type "Key Structure" :default "AnyKey"))
  ;[1 1 1] Primary weapon fire control
  (:`Pressed`
    (set `self.Fire_1_Pressed` true)
    (`/Game/Blueprints/Weapons/BP_WeaponBase.FireBeam` (`self.BP_BeamCannon1`))
    (`/Game/Blueprints/Weapons/BP_WeaponBase.FireBeam` (`self.BP_BeamCannon2`)))
  (:`Released`
    (set `self.Fire_1_Pressed` false)
    (`/Game/Blueprints/Weapons/BP_BeamCannon.StopFiring` (`self.BP_BeamCannon1`))
    (`/Game/Blueprints/Weapons/BP_BeamCannon.StopFiring` (`self.BP_BeamCannon2`))))

(fn `AddMouseInputToHUD`
  (bind _hud_steeringwidget (`self.HUD_SteeringWidget`))
  (bind _maxradius (`/Game/Blueprints/UI/HUD/HUD_SteeringIndicator.MaxRadius` _hud_steeringwidget))
  (bind _returnvalue (- 0.0 _maxradius))
  (set `/Game/Blueprints/UI/HUD/HUD_SteeringIndicator.SteerX` (`KismetMathLibrary.FClamp` (+ (`/Game/Blueprints/UI/HUD/HUD_SteeringIndicator.SteerX` _hud_steeringwidget) (* (`self.GetInputAxisValue`) (`self.HUD_MouseSteeringSpeed`))) _returnvalue _maxradius) _hud_steeringwidget)
  (set `/Game/Blueprints/UI/HUD/HUD_SteeringIndicator.SteerY` (`KismetMathLibrary.FClamp` (- (`/Game/Blueprints/UI/HUD/HUD_SteeringIndicator.SteerY` _hud_steeringwidget) (* (`self.GetInputAxisValue`) (`self.HUD_MouseSteeringSpeed`))) _returnvalue _maxradius) _hud_steeringwidget))

(fn `GetScreenSpaceAimPoint`
  (returns (screenPos :type "Vector2D Structure"))
  (return (`GameplayStatics.ProjectWorldToScreen` (`GameplayStatics.GetPlayerController` 0) (+ (`SceneComponent.GetSocketLocation` (`self.transmorpher`) "NeckSocket_VehicleModeHardpoint") (* (`self.GetActorForwardVector`) 50000.0)))))

(fn `SetRibbonVelocity`
  (params (Delta :type "Float (double-precision)")))

(fn `UserConstructionScript`)